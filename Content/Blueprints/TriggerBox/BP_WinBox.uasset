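; BP_WinBox is a trigger box that ends the level in victory when a BP_MyCharacter overlaps it.
; On overlap it shows a French win message with the character's score through the HUD, then stops movement and disables player input.
; It then saves the best score through the GI_MyGame game instance and opens the MainMenu level after a short delay.
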(event OnComponentBeginOverlap(Box)
  (params (OverlappedComponent :type Primitive%20Component%20Object%20Reference) (OtherActor :type Actor%20Object%20Reference) (OtherComp :type Primitive%20Component%20Object%20Reference) (OtherBodyIndex :type Integer) (bFromSweep :type Boolean) (SweepResult :type Hit%20Result%20Structure%20%28by%20ref%29))
  (bind _asbp_my_character (Utilities|Casting|CastToBP_MyCharacter OtherActor))
  (Variables|/Game/Blueprints/Player/BP_MyCharacter.BP_MyCharacter_C|SetMessageToDisplay _asbp_my_character (Utilities|Text|FormatText "Vous avez gagné 
Score: {Score}" (Variables|/Game/Blueprints/Player/BP_MyCharacter.BP_MyCharacter_C|GetScore _asbp_my_character)))
  (Default|DisplayMessageBox (Variables|/Game/Blueprints/Player/BP_MyCharacter.BP_MyCharacter_C|GetHUDRef _asbp_my_character))
  (Components|Movement|StopMovementImmediately (Variables|/Script/Engine.Character|GetCharacterMovement _asbp_my_character))
  (Input|DisableInput (Game|GetPlayerCharacter 0) (Game|GetPlayerController 0))
  (bind _asgi_my_game (Utilities|Casting|CastToGI_MyGame (Game|GetGameInstance)))
  (Default|SaveBestScore _asgi_my_game)
  (Utilities|FlowControl|Delay 5.0)
  (Game|OpenLevel(byName) "MainMenu"))

(fn ConstructionScript)