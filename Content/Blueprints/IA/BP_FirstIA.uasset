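; BP_FirstIA is a simple AI pawn that chases the player character when the player is nearby.
; A Sphere component's overlap events, filtered to BP_MyCharacter, set and clear an IsThePlayerNearMe flag.
; While the flag is true, Tick calls AIMoveTo toward player character 0 every frame, using a small acceptance radius.
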(event OnComponentBeginOverlap(Sphere)
  (params (OverlappedComponent :type Primitive%20Component%20Object%20Reference) (OtherActor :type Actor%20Object%20Reference) (OtherComp :type Primitive%20Component%20Object%20Reference) (OtherBodyIndex :type Integer) (bFromSweep :type Boolean) (SweepResult :type Hit%20Result%20Structure%20%28by%20ref%29))
  (Utilities|Casting|CastToBP_MyCharacter OtherActor)
  (Variables|Default|SetIsThePlayerNearMe? true))

(event OnComponentEndOverlap(Sphere)
  (params (OverlappedComponent :type Primitive%20Component%20Object%20Reference) (OtherActor :type Actor%20Object%20Reference) (OtherComp :type Primitive%20Component%20Object%20Reference) (OtherBodyIndex :type Integer))
  (Utilities|Casting|CastToBP_MyCharacter OtherActor)
  (Variables|Default|SetIsThePlayerNearMe? false))

(event EventTick
  (params (DeltaSeconds :type Float%20%28single-precision%29))
  (if (Variables|Default|GetIsThePlayerNearMe?)
    (AI|AIMoveTo self "0, 0, 0" (Game|GetPlayerCharacter 0) 5e+01 false)))

(fn ConstructionScript)