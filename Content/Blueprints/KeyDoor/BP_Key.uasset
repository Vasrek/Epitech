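; BP_Key is a colored key pickup that the player character collects by touching it.
; The construction script sets the material on the Sphere mesh from the KeyColor value of yellow, blue, red or green.
; When BP_MyCharacter begins overlapping Sphere1, the key passes its KeyColor to the character's AddKey and destroys itself.
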(event OnComponentBeginOverlap(Sphere1)
  (params (OverlappedComponent :type Primitive%20Component%20Object%20Reference) (OtherActor :type Actor%20Object%20Reference) (OtherComp :type Primitive%20Component%20Object%20Reference) (OtherBodyIndex :type Integer) (bFromSweep :type Boolean) (SweepResult :type Hit%20Result%20Structure%20%28by%20ref%29))
  (bind _asbp_my_character (Utilities|Casting|CastToBP_MyCharacter OtherActor))
  (Default|AddKey _asbp_my_character (Variables|Default|GetKeyColor))
  (Actor|DestroyActor))

(fn ConstructionScript
  (switch Utilities|FlowControl|Switch|SwitchonE_Door_Key_ColorSystem (Variables|Default|GetKeyColor)
    (:NewEnumerator0
      (Variables|Default|SetMaterial "/Engine/EngineMaterials/CubeMaterial.CubeMaterial"))
    (:NewEnumerator1
      (Variables|Default|SetMaterial "/AnimationSharing/AnimSharingBlue.AnimSharingBlue"))
    (:NewEnumerator2
      (Variables|Default|SetMaterial "/AnimationSharing/AnimSharingRed.AnimSharingRed"))
    (:NewEnumerator3
      (Variables|Default|SetMaterial "/AnimationSharing/AnimSharingGreen.AnimSharingGreen")))
  (Rendering|Material|SetMaterial (Variables|Default|GetSphere) 0 (Variables|Default|GetMaterial)))