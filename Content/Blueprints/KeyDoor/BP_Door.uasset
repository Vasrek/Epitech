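; Color-coded door that opens when the player character enters its trigger box carrying the matching key color.
; The Construction Script sets the cube's material from DoorColor.
; A match consumes the key, calls CallDoorOpening and starts a looping timer that sinks the cube with FInterpTo until near its lowered target.
; A mismatch notifies the character of the required color, and leaving the box hides the HUD message.
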(event OnComponentBeginOverlap(box)
  (params (OverlappedComponent :type Primitive%20Component%20Object%20Reference) (OtherActor :type Actor%20Object%20Reference) (OtherComp :type Primitive%20Component%20Object%20Reference) (OtherBodyIndex :type Integer) (bFromSweep :type Boolean) (SweepResult :type Hit%20Result%20Structure%20%28by%20ref%29))
  (bind _doorcolor (Variables|Default|GetDoorColor))
  (bind _asbp_my_character (Utilities|Casting|CastToBP_MyCharacter OtherActor))
  (if (Utilities|Enum|Equal(Enum) (Variables|/Game/Blueprints/Player/BP_MyCharacter.BP_MyCharacter_C|GetCurrentKeyColor _asbp_my_character) _doorcolor)
    (CallFunction|OpenDoor)
    (Variables|/Game/Blueprints/Player/BP_MyCharacter.BP_MyCharacter_C|SetCurrentKeyColor _asbp_my_character "NewEnumerator4")
    (else
      (Default|DontHavetheRightKey _asbp_my_character _doorcolor))))

(event OnComponentEndOverlap(box)
  (params (OverlappedComponent :type Primitive%20Component%20Object%20Reference) (OtherActor :type Actor%20Object%20Reference) (OtherComp :type Primitive%20Component%20Object%20Reference) (OtherBodyIndex :type Integer))
  (bind _asbp_my_character (Utilities|Casting|CastToBP_MyCharacter OtherActor))
  (Default|HideMessageBox (Variables|/Game/Blueprints/Player/BP_MyCharacter.BP_MyCharacter_C|GetHUDRef _asbp_my_character)))

(event Custom|OpenDoor
  (Utilities|Time|SetTimerbyFunctionName 0 "FOpenDoor" 0.01 true)
  (Default|CallDoorOpening))

(event EventBeginPlay
  (bind _output_get (Variables|Default|SetDefaultZVlaue (.z (Transformation|GetWorldLocation (Variables|Default|GetCube)))))
  (Variables|Default|SetTargetOpenDoorZValue (- _output_get 5e+02)))

(fn ConstructionScript
  (switch Utilities|FlowControl|Switch|SwitchonE_Door_Key_ColorSystem (Variables|Default|GetDoorColor)
    (:NewEnumerator0
      (Variables|Default|SetMaterial "/Engine/EngineMaterials/CubeMaterial.CubeMaterial"))
    (:NewEnumerator1
      (Variables|Default|SetMaterial "/AnimationSharing/AnimSharingBlue.AnimSharingBlue"))
    (:NewEnumerator2
      (Variables|Default|SetMaterial "/AnimationSharing/AnimSharingRed.AnimSharingRed"))
    (:NewEnumerator3
      (Variables|Default|SetMaterial "/AnimationSharing/AnimSharingGreen.AnimSharingGreen")))
  (Rendering|Material|SetMaterial (Variables|Default|GetCube) 0 (Variables|Default|GetMaterial)))

(fn FOpenDoor
  (bind _returnvalue (Utilities|Time|GetWorldDeltaSeconds))
  (bind _cube (Variables|Default|GetCube))
  (bind _targetopendoorzvalue (Variables|Default|GetTargetOpenDoorZValue))
  (bind _returnvalue_2 (Transformation|GetWorldLocation _cube))
  (bind _returnvalue_3 (Math|Interpolation|FInterpTo (.z _returnvalue_2) _targetopendoorzvalue _returnvalue 0.5))
  (Transformation|SetWorldLocation (Variables|Default|GetCube) (Math|Vector|MakeVector (.x _returnvalue_2) (.y _returnvalue_2) _returnvalue_3) false false)
  (if (Math|Float|NearlyEqual(Float) _returnvalue_3 _targetopendoorzvalue 5.0)
    (Utilities|Time|ClearTimerbyFunctionName 0 "FOpenDoor")))