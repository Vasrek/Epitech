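; BP_KeyInteract is a colored key pickup that offers itself to the player character for interaction.
; Overlapping its sphere shows the HUD message box, sets a color-specific pickup prompt, enables interaction and registers the key with BP_MyCharacter.
; Leaving hides the box and disables interaction, without unregistering the key.
; The construction script sets the Sphere mesh material from KeyColor; the pickup itself is handled outside this Blueprint.
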(event OnComponentBeginOverlap(Sphere1)
  (params (OverlappedComponent :type Primitive%20Component%20Object%20Reference) (OtherActor :type Actor%20Object%20Reference) (OtherComp :type Primitive%20Component%20Object%20Reference) (OtherBodyIndex :type Integer) (bFromSweep :type Boolean) (SweepResult :type Hit%20Result%20Structure%20%28by%20ref%29))
  (bind _asbp_my_character (Utilities|Casting|CastToBP_MyCharacter OtherActor))
  (Variables|/Game/Blueprints/Player/BP_MyCharacter.BP_MyCharacter_C|SetCanInteract? _asbp_my_character true)
  (Default|DisplayMessageBox (Variables|/Game/Blueprints/Player/BP_MyCharacter.BP_MyCharacter_C|GetHUDRef _asbp_my_character))
  (Variables|/Game/Blueprints/Player/BP_MyCharacter.BP_MyCharacter_C|SetMessageToDisplay _asbp_my_character (Utilities|Text|FormatText "Press E (keyboard) X (xbox) to pick up KEY {color}" (Utilities|Select :Index (Variables|Default|GetKeyColor) :NewEnumerator4 "None" :NewEnumerator0 "Yellow" :NewEnumerator1 "Blue" :NewEnumerator2 "Red" :NewEnumerator3 "Green")))
  (Default|AddInteractItem _asbp_my_character self))

(event OnComponentEndOverlap(Sphere1)
  (params (OverlappedComponent :type Primitive%20Component%20Object%20Reference) (OtherActor :type Actor%20Object%20Reference) (OtherComp :type Primitive%20Component%20Object%20Reference) (OtherBodyIndex :type Integer))
  (bind _asbp_my_character (Utilities|Casting|CastToBP_MyCharacter OtherActor))
  (Default|HideMessageBox (Variables|/Game/Blueprints/Player/BP_MyCharacter.BP_MyCharacter_C|GetHUDRef _asbp_my_character))
  (Variables|/Game/Blueprints/Player/BP_MyCharacter.BP_MyCharacter_C|SetCanInteract? _asbp_my_character false))

(fn ConstructionScript
  (switch Utilities|FlowControl|Switch|SwitchonE_Door_Key_ColorSystem (Variables|Default|GetKeyColor)
    (:NewEnumerator0
      (Variables|Default|SetMaterial "/Engine/EngineMaterials/CubeMaterial.CubeMaterial"))
    (:NewEnumerator1
      (Variables|Default|SetMaterial "/AnimationSharing/AnimSharingBlue.AnimSharingBlue"))
    (:NewEnumerator2
      (Variables|Default|SetMaterial "/AnimationSharing/AnimSharingRed.AnimSharingRed"))
    (:NewEnumerator3
      (Variables|Default|SetMaterial "/AnimationSharing/AnimSharingGreen.AnimSharingGreen")))
  (Rendering|Material|SetMaterial (Variables|Default|GetSphere) 0 (Variables|Default|GetMaterial)))