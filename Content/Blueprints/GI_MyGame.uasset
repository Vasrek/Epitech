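; Game instance Blueprint that persists the player's best score in a single SG_Player save slot.
; CreateSaveGame loads the existing save into SaveGameRef and BestScore, or creates and writes a new one.
; SaveBestScore compares the character's Score with a freshly loaded save, but writes any higher value to the cached SaveGameRef.
; It prints the result and saves that cached object either way, without updating BestScore.
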(event Custom|LoadBestScore
  (bind _returnvalue (SaveGame|LoadGamefromSlot (Variables|Default|GetSaveSlotName)))
  (bind _assg_player (Utilities|Casting|CastToSG_Player _returnvalue))
  (Variables|Default|SetBestScore (Variables|/Game/Blueprints/Save/SG_Player.SG_Player_C|Getscore _assg_player))
  (Variables|Default|SetSaveGameRef _assg_player))

(event Custom|SaveBestScore
  (bind _returnvalue (SaveGame|LoadGamefromSlot (Variables|Default|GetSaveSlotName)))
  (bind _assg_player (Utilities|Casting|CastToSG_Player _returnvalue))
  (bind _asbp_my_character (Utilities|Casting|CastToBP_MyCharacter (Game|GetPlayerCharacter 0)))
  (if (> (Variables|/Game/Blueprints/Player/BP_MyCharacter.BP_MyCharacter_C|GetScore _asbp_my_character) (Variables|/Game/Blueprints/Save/SG_Player.SG_Player_C|Getscore _assg_player))
    (bind _output_get (Variables|/Game/Blueprints/Save/SG_Player.SG_Player_C|Setscore (Variables|Default|GetSaveGameRef) (Variables|/Game/Blueprints/Player/BP_MyCharacter.BP_MyCharacter_C|GetScore _asbp_my_character)))
    (Development|PrintString (Utilities|String|Append "New Best Score saved : " (Utilities|String|ToString(Integer) _output_get)))
    (else
      (Development|PrintString (Utilities|String|Append "No new Best Score to save previous score: " (Utilities|String|ToString(Integer) (Variables|/Game/Blueprints/Save/SG_Player.SG_Player_C|Getscore _assg_player))))))
  (SaveGame|SaveGametoSlot (Variables|Default|GetSaveGameRef) (Variables|Default|GetSaveSlotName)))

(event Custom|CreateSaveGame
  (bind _returnvalue (SaveGame|DoesSaveGameExist (Variables|Default|GetSaveSlotName)))
  (if _returnvalue
    (CallFunction|LoadBestScore)
    (else
      (bind _returnvalue_2 (SaveGame|CreateSaveGameObject "/Game/Blueprints/Save/SG_Player.SG_Player_C"))
      (bind _output_get (Variables|Default|SetSaveGameRef _returnvalue_2))
      (SaveGame|SaveGametoSlot _output_get (Variables|Default|GetSaveSlotName)))))