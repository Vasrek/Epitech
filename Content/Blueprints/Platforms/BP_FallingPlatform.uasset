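; BP_FallingPlatform is a platform that drops after the player character steps into its trigger box, then resets itself.
; BeginPlay saves the Cube's world transform as the home position.
; An overlap by BP_MyCharacter starts a short delay, then enables physics simulation on the Cube so it falls.
; After a second delay, it disables physics and teleports the Cube back to the saved transform.
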(event OnComponentBeginOverlap(Box)
  (params (OverlappedComponent :type Primitive%20Component%20Object%20Reference) (OtherActor :type Actor%20Object%20Reference) (OtherComp :type Primitive%20Component%20Object%20Reference) (OtherBodyIndex :type Integer) (bFromSweep :type Boolean) (SweepResult :type Hit%20Result%20Structure%20%28by%20ref%29))
  (Utilities|Casting|CastToBP_MyCharacter OtherActor)
  (Utilities|FlowControl|Delay 2.0)
  (Physics|SetSimulatePhysics (Variables|Default|GetCube) true)
  (Utilities|FlowControl|Delay 3.0)
  (Physics|SetSimulatePhysics (Variables|Default|GetCube) false)
  (Transformation|SetWorldTransform (Variables|Default|GetCube) (Variables|Default|GetMyDefaultTransform) false true))

(event EventBeginPlay
  (Variables|Default|SetMyDefaultTransform (Transformation|GetWorldTransform (Variables|Default|GetCube))))

(fn ConstructionScript)