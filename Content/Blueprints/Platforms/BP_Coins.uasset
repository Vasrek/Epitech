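; BP_Coins is a collectible coin that spins and awards score to the player.
; Tick adds RotationSpeed to the Sphere's world roll every frame, without delta-time scaling.
; Overlapping Sphere1 with a BP_MyCharacter adds 25 score, plays the CompileSuccess 2D sound, and destroys the coin.
; A node that would randomize RotationSpeed is disconnected, so it never runs.
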(event OnComponentBeginOverlap(Sphere1)
  (params (OverlappedComponent :type Primitive%20Component%20Object%20Reference) (OtherActor :type Actor%20Object%20Reference) (OtherComp :type Primitive%20Component%20Object%20Reference) (OtherBodyIndex :type Integer) (bFromSweep :type Boolean) (SweepResult :type Hit%20Result%20Structure%20%28by%20ref%29))
  (bind _asbp_my_character (Utilities|Casting|CastToBP_MyCharacter OtherActor))
  (Default|AddScore _asbp_my_character 25)
  (Audio|PlaySound2D "/Engine/EditorSounds/Notifications/CompileSuccess.CompileSuccess" 1.0 1.0 0.0 0 0)
  (Actor|DestroyActor))

(event EventTick
  (params (DeltaSeconds :type Float%20%28single-precision%29))
  (bind _sphere (Variables|Default|GetSphere))
  (bind _returnvalue (Transformation|GetWorldRotation _sphere))
  (Transformation|SetWorldRotation _sphere (Math|Rotator|MakeRotator (+ (.roll _returnvalue) (Variables|Default|GetRotationSpeed)) (.pitch _returnvalue) (.yaw _returnvalue)) false false))

(event EventBeginPlay)

(fn ConstructionScript)